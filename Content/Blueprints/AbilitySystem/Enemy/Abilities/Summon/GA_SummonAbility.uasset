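; Enemy summon gameplay ability that currently previews spawn points with debug spheres rather than spawning any actors.
; On activation it stores the result of GetSpawnLocations and shuffles the array to randomize order.
; A delay-driven index loop draws one short-lived sphere per location at a staggered interval, then ends the ability.
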(event Ability|EventActivateAbility
  (Variables|Default|SetSpawnLocationIndex 0)
  (bind _returnvalue (Class|AuraSummonAbility|GetSpawnLocations))
  (bind _output_get (Variables|Default|SetSpawnLocations _returnvalue))
  (Utilities|Array|Shuffle _output_get)
  (if (< (Variables|Default|GetSpawnLocationIndex) (Utilities|Array|Length (Variables|Default|GetSpawnLocations))) :!label _label
    (Rendering|Debug|DrawDebugSphere (Utilities|Array|Get(acopy) (Variables|Default|GetSpawnLocations) (Variables|Default|GetSpawnLocationIndex)) 25.0 12 "(R=1.000000,G=0.440625,B=0.679210,A=1.000000)" 2.0)
    (Variables|Default|SetSpawnLocationIndex (+ (Variables|Default|GetSpawnLocationIndex) 1))
    (Utilities|FlowControl|Delay 0.2)
    (goto _label)
    (else
      (Ability|EndAbility))))

(event Ability|EventOnEndAbility
  (params (bWasCancelled :type Boolean)))