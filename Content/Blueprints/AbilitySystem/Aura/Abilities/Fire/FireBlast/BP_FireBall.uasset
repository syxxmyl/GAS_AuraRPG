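; Fire Blast fireball projectile that flies out from its spawn point, returns to a target actor and explodes near it.
; On the server, an outgoing timeline lerps it forward to an apex set by the travel distance.
; A returning timeline then lerps it toward the actor's live location, calling the hit handler and applying explosion damage once within explode distance.
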(event EventStartOutgoingTimeline
  (Networking|SwitchHasAuthority
    (:Authority
      (Variables|Default|SetInitialLocation (Transformation|GetActorLocation))
      (Variables|Default|SetApexLocation (+ (Variables|Default|GetInitialLocation) (* (Transformation|GetActorForwardVector) (Variables|Default|GetTravelDistance))))
      (bind _outgoingtrack (Timeline|OutgoingTimeLine Play)
        (:Update
          (Transformation|SetActorLocation (Math|Vector|Lerp(Vector) (Variables|Default|GetInitialLocation) (Variables|Default|GetApexLocation) _outgoingtrack) false false))
        (:Finished
          (bind _returningtrack (Timeline|ReturningTimeLine Play)
            (:Update
              (Transformation|SetActorLocation (Math|Vector|Lerp(Vector) (Variables|Default|GetApexLocation) (Transformation|GetActorLocation (Variables|Default|GetReturnToActor)) _returningtrack) false false)
              (bind _returnvalue (CallFunction|IsWithinExplodeDistance))
              (if _returnvalue
                (Class|AuraProjectile|OnHit)
                (Class|AuraFireBall|ApplyExplosionDamage)))))))))

(fn ConstructionScript)

(fn IsWithinExplodeDistance
  (return (< (Math|Vector|VectorLength (- (Transformation|GetActorLocation) (Transformation|GetActorLocation (Variables|Default|GetReturnToActor)))) (Variables|Default|GetExplodeDistance))))