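; BP_Aura_MainMenu is a display version of the Aura character, named for the main menu, that animates a fireball and a magic circle.
; BeginPlay caches the FireBall's world location as the base for a sine-wave vertical bob scaled by Amplitude.
; Tick advances a Time accumulator through UpdateTime, which resets near two pi, and spins the MagicCircleDecal around its roll axis at MagicCircleRotationRate.
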(event EventBeginPlay
  (Variables|Default|SetFireBallInitialLocation (Transformation|GetWorldLocation (Variables|Default|GetFireBall))))

(event EventTick
  (params (DeltaSeconds :type Float%20%28single-precision%29))
  (CallFunction|UpdateTime DeltaSeconds)
  (Transformation|SetWorldLocation (Variables|Default|GetFireBall) (+ (Variables|Default|GetFireBallInitialLocation) (Math|Vector|MakeVector 0.0 0.0 (* (Math|Trig|Sin(Radians) (Variables|Default|GetTime)) (Variables|Default|GetAmplitude)))) false false)
  (Transformation|AddLocalRotation (Variables|Default|GetMagicCircleDecal) (Math|Rotator|MakeRotator (* (Utilities|Time|GetWorldDeltaSeconds) (Variables|Default|GetMagicCircleRotationRate)) 0.0 0.0) false false))

(fn ConstructionScript)

(fn UpdateTime
  (params (DeltaSeconds :type Float%20%28double-precision%29))
  (bind _output_get (Variables|Default|SetTime (+ DeltaSeconds (Variables|Default|GetTime))))
  (if (> _output_get 6.28)
    (Variables|Default|SetTime 0.0)))