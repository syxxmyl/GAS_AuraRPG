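; Base pickup actor that plays a spawn animation, rising and scaling before it begins its idle motion.
; On BeginPlay a timeline drives uniform scale and a height offset from InitialLocation, scaled by SpawnApex, then calls StartSinusoidalMovement and StartRotation when finished.
; Tick applies the cached CalculatedLocation and CalculatedRotation to the actor every frame, separating motion calculation from transform updates.
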(event EventBeginPlay
  (bind (_direction _elevation _scale) (Timeline|PickupElevationTimeline Play)
    (:Update
      (Variables|Default|SetCalculatedLocation (Math|Vector|MakeVector (.InitialLocation_X (CallFunction|SetCalculateLocation _elevation)) (.InitialLocation_Y (CallFunction|SetCalculateLocation _elevation)) (.ReturnValue (CallFunction|SetCalculateLocation _elevation))))
      (Transformation|SetActorScale3D (Math|Vector|MakeVector _scale _scale _scale)))
    (:Finished
      (Class|AuraEffectActor|StartSinusoidalMovement)
      (Class|AuraEffectActor|StartRotation))))

(event EventTick
  (params (DeltaSeconds :type Float%20%28single-precision%29))
  (Transformation|SetActorLocation (Variables|Default|GetCalculatedLocation) false false)
  (Transformation|SetActorRotation (Variables|Default|GetCalculatedRotation)))

(fn ConstructionScript)

(fn SetCalculateLocation
  (params (A :type Float%20%28double-precision%29))
  (bind _initiallocation (Variables|Default|GetInitialLocation))
  (return (.x _initiallocation) (.y _initiallocation) (+ (.z _initiallocation) (* A (Variables|Default|GetSpawnApex)))))